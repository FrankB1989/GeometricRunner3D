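; Base player pawn for a lane-based game, with left/right lane switching, a jump and an obstacle-hit death.
; BeginPlay takes lane count and width from the Level Manager and finds the tagged end camera.
; Timelines drive lane lerps and a physics-free jump of the Player component, with Tick starting the trail during play.
; HitObstacle blends to the end camera, hides the player, stops the trail and spawns an explosion.
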(event EventBeginPlay
  (CallFunction|Initialize))

(event EventTick
  (params (DeltaSeconds :type Float%20%28single-precision%29))
  ;[1 1 1] Branch used to activate particle system when start the game
  (if (and (not (Components|Activation|IsActive (Variables|Default|GetTrail))) (Variables|/Game/Blueprints/BP_LevelManager.BP_LevelManager_C|GetIsPlaying? (Variables|Default|GetLevelManagerRef)))
    (Components|Activation|Activate (Variables|Default|GetTrail) false)))

(event Input|ActionEvents|InputActionLeft
  (params (Key :type Key%20Structure :default "None"))
  (bind _returnvalue (Transformation|GetActorLocation))
  ;[1 1 1] Move Left And Right Logic
  (:Pressed
    (if (Variables|/Game/Blueprints/BP_LevelManager.BP_LevelManager_C|GetIsPlaying? (Variables|Default|GetLevelManagerRef))
      (if (not (<= (Variables|Default|GetCurrentLane) 1))
        (if (not (Variables|Default|GetIsMoving?))
          (Variables|Default|SetIsMoving? true)
          (Variables|Default|SetTargetPosition (- (.y (Transformation|GetActorLocation)) (Variables|Default|GetLaneWidthRef)))
          (bind _movetimelineparameter (Timeline|MoveLeft PlayFromStart)
            (:Update
              (Transformation|SetActorLocation (Math|Vector|MakeVector (.x _returnvalue) (Math|Float|Lerp (.y _returnvalue) (Variables|Default|GetTargetPosition) _movetimelineparameter) (.z _returnvalue)) false false))
            (:Finished
              (Variables|Default|SetIsMoving? false)
              (Math|Integer|DecrementInt (Variables|Default|GetCurrentLane)))))))))

(event Input|ActionEvents|InputActionRight
  (params (Key :type Key%20Structure :default "None"))
  (bind _returnvalue (Transformation|GetActorLocation))
  ;[1 1 1] Move Left And Right Logic
  (:Pressed
    (if (Variables|/Game/Blueprints/BP_LevelManager.BP_LevelManager_C|GetIsPlaying? (Variables|Default|GetLevelManagerRef))
      (if (not (== (Variables|Default|GetCurrentLane) (Variables|/Game/Blueprints/BP_LevelManager.BP_LevelManager_C|GetNumberOfLanes (Variables|Default|GetLevelManagerRef))))
        (if (not (Variables|Default|GetIsMoving?))
          (Variables|Default|SetTargetPosition (+ (.y (Transformation|GetActorLocation)) (Variables|Default|GetLaneWidthRef)))
          (bind _moverightparameter (Timeline|MoveRightTimeline PlayFromStart)
            (:Update
              (Transformation|SetActorLocation (Math|Vector|MakeVector (.x _returnvalue) (Math|Float|Lerp (.y _returnvalue) (Variables|Default|GetTargetPosition) _moverightparameter) (.z _returnvalue)) false false))
            (:Finished
              (Variables|Default|SetIsMoving? false)
              (Math|Integer|IncrementInt (Variables|Default|GetCurrentLane)))))))))

(event Input|ActionEvents|InputActionJump
  (params (Key :type Key%20Structure :default "None"))
  (bind _returnvalue (Transformation|GetActorLocation))
  ;[1 1 1] Jump Action
  (:Pressed
    (if (not (Variables|Default|GetIsMoving?))
      (Variables|Default|SetIsMoving? true)
      (bind _jumpcurve (Timeline|JumpWithoutPhysics PlayFromStart)
        (:Update
          (Transformation|SetWorldLocation (Variables|Default|GetPlayer) (Math|Vector|MakeVector (.x _returnvalue) (.y _returnvalue) (Math|Float|Clamp(Float) (* _jumpcurve (.z _returnvalue)) (.z _returnvalue) 5e+02)) false false))
        (:Finished
          (Variables|Default|SetIsMoving? false))))))

(fn ConstructionScript)

(fn Initialize
  (bind _output (Utilities|GetLevelManager)
    (:Is%20Valid
      (Variables|Default|SetLevelManagerRef _output)
      (Variables|Default|SetCurrentLane (+ (/ (Variables|/Game/Blueprints/BP_LevelManager.BP_LevelManager_C|GetNumberOfLanes (Variables|Default|GetLevelManagerRef)) 2) 1))
      (Variables|Default|SetLaneWidthRef (Variables|/Game/Blueprints/BP_LevelManager.BP_LevelManager_C|GetLaneWidth (Variables|Default|GetLevelManagerRef)))
      (bind _outactors (Actor|GetAllActorswithTag "EndCamera"))
      (Variables|Default|SetEndCameraActorRef (Utilities|Array|Get(acopy) _outactors)))
    (:Is%20Not%20Valid
      (Development|PrintString "No Level Manager Find in Project"))))

(fn HitObstacle
  ;[1 1 1] Hit Obstacle Function with all the logic
  (bind _endcameraactorref (Variables|Default|GetEndCameraActorRef)
    (:then
      (Game|Player|SetViewTargetwithBlend (Game|GetPlayerController 0) _endcameraactorref 1.5 "VTBlend_Linear" 0.0 false))
    (:else
      _))
  (Rendering|ToggleVisibility (Variables|Default|GetPlayer) false)
  (Components|Activation|Deactivate (Variables|Default|GetTrail))
  (Effects|SpawnEmitteratLocation "/Game/StarterContent/Particles/P_Explosion.P_Explosion" (Transformation|GetActorLocation)))