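; BP_TunnelObstacle is a tunnel obstacle that ends the game when the player hits it.
; On static mesh overlap with a BP_PlayerPawnBase, it calls HitObstacle on the pawn, then GameOver on the level manager if valid.
; The construction script randomizes the mesh's Y scale for size variation, keeping X and Z fixed.
; SetParent and ReturnParent store and expose a reference to a parent.
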(event OnComponentBeginOverlap(StaticMesh)
  (params (OverlappedComponent :type Primitive%20Component%20Object%20Reference) (OtherActor :type Actor%20Object%20Reference) (OtherComp :type Primitive%20Component%20Object%20Reference) (OtherBodyIndex :type Integer) (bFromSweep :type Boolean) (SweepResult :type Hit%20Result%20Structure%20%28by%20ref%29))
  ;[1 1 1] Call Game Over When Hit Player
  (bind _asbp_player_pawn_base (Utilities|Casting|CastToBP_PlayerPawnBase OtherActor))
  (Default|HitObstacle _asbp_player_pawn_base)
  (bind _output (Utilities|GetLevelManager)
    (:Is%20Valid
      (Default|GameOver _output))))

(fn ConstructionScript
  (Transformation|SetWorldScale3D (Variables|Default|GetStaticMesh) (Math|Vector|MakeVector 0.8 (Math|Random|RandomFloatinRange 1.0 1.5) 0.8)))

(fn ReturnParent
  (return (Variables|Default|GetParentRef)))

(fn SetParent
  (params (Parent :type BP%20Spawner%20Base%20Object%20Reference))
  (Variables|Default|SetParentRef Parent)
  (return false))