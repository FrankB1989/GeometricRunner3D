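; BPC_ScrollingComponent is an actor component that scrolls its owning actor at the level's speed.
; On BeginPlay it caches the Level Manager reference when the lookup returns a valid result.
; Each tick it scales the owner's forward vector by the manager's LevelSpeed and delta time, then applies it as a local-space offset without sweep.
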(event EventBeginPlay
  (bind (_levelmanager _isvalid_) (CallFunction|GetLevelManagerFunction))
  (if _isvalid_
    (Variables|Default|SetLevelManagerRef _levelmanager)))

(event EventTick
  (params (DeltaSeconds :type Float%20%28single-precision%29))
  (Variables|Default|SetDeltaSeconds DeltaSeconds)
  (bind _output_get (Variables|Default|SetForwardVectorMovement (* (* (Transformation|GetActorForwardVector (Components|GetOwner)) (Variables|/Game/Blueprints/BP_LevelManager.BP_LevelManager_C|GetLevelSpeed (Variables|Default|GetLevelManagerRef))) (Variables|Default|GetDeltaSeconds))))
  (Transformation|AddActorLocalOffset (Components|GetOwner) _output_get false false))