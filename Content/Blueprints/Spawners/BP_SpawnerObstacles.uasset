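; Obstacle spawner that periodically spawns obstacles at its own location while the level manager reports the game is playing.
; On BeginPlay it caches the level manager, spawns immediately, then starts a looping timer whose random interval is rolled once.
; It overrides the parent's SpawnActor to avoid origin spawns that instantly overlap the player and end the game.
; Each obstacle receives the spawner as parent; actors reported out of bounds are destroyed.
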(event Custom|LineUpNextObstaclesSpawn
  (if (Variables|/Game/Blueprints/BP_LevelManager.BP_LevelManager_C|GetIsPlaying? (Variables|Default|GetLevelManagerRef))
    (CallFunction|PlaceObstacles)))

(event EventBeginPlay
  (bind (_levelmanager _isvalid_) (CallFunction|GetLevelManagerFunction))
  (if _isvalid_
    (Variables|Default|SetLevelManagerRef _levelmanager)
    (CallFunction|LineUpNextObstaclesSpawn)
    (Utilities|Time|SetTimerbyEvent (delegate Custom|LineUpNextObstaclesSpawn) (Math|Random|RandomFloatinRange (Variables|Default|GetMinDelay) (Variables|Default|GetMaxDelay)) true)))

(event EventSpawnedActorHitBounds
  (params (ActorOutOfBounds :type Actor%20Object%20Reference))
  (Actor|DestroyActor ActorOutOfBounds))

(fn ConstructionScript
  (|CallParentFunction))

(fn PlaceObstacles
  (bind _returnvalue (Transformation|GetActorLocation))
  (bind _actorspawned (CallFunction|SpawnActor))
  (Transformation|SetActorLocation _actorspawned (Math|Vector|MakeVector (.x _returnvalue) (.y _returnvalue) (.z _returnvalue)) false false))

(fn SpawnActor
  ;[1 1 1] Override the base function because if the obstacle is spawned in 0 0 0 location it overlap the player when spawn and end the game immediately
  (bind _returnvalue (Game|SpawnActorfromClass (Variables|Default|GetActorTypeToSpawn) (Math|Transform|MakeTransform (Transformation|GetActorLocation) "0, 0, 0" "1,1,1") "Undefined" 0 0))
  (Class|BPISpawnable|SetParent(Message) _returnvalue self)
  (return _returnvalue))