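; BP_SpawnerCoin is a spawner that places coins at its own location while the level is playing.
; BeginPlay makes an immediate attempt, then starts a looping timer with one random delay between MinDelay and MaxDelay, which is never re-rolled.
; Each attempt checks the level manager, spawns ActorTypeToSpawn through an overridden SpawnActor that passes the spawner as parent, then raises the coin slightly.
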(event Custom|LineUpNextCoin
  (bind _output (Utilities|GetLevelManager)
    (:Is%20Valid
      (if (Variables|/Game/Blueprints/BP_LevelManager.BP_LevelManager_C|GetIsPlaying? _output)
        (CallFunction|PlaceCoin)))))

(event EventBeginPlay
  (CallFunction|LineUpNextCoin)
  (Utilities|Time|SetTimerbyEvent (delegate Custom|LineUpNextCoin) (Math|Random|RandomFloatinRange (Variables|Default|GetMinDelay) (Variables|Default|GetMaxDelay)) true))

(event Collision|EventActorBeginOverlap
  (params (OtherActor :type Actor%20Object%20Reference)))

(event EventTick
  (params (DeltaSeconds :type Float%20%28single-precision%29)))

(fn ConstructionScript
  (|CallParentFunction))

(fn PlaceCoin
  (bind _returnvalue (Transformation|GetActorLocation))
  (bind _actorspawned (CallFunction|SpawnActor))
  (Transformation|SetActorLocation _actorspawned (Math|Vector|MakeVector (.x _returnvalue) (.y _returnvalue) (+ (.z _returnvalue) 5e+01)) false false))

(fn SpawnActor
  (bind _returnvalue (Game|SpawnActorfromClass (Variables|Default|GetActorTypeToSpawn) (Math|Transform|MakeTransform (Transformation|GetActorLocation) "0, 0, 0" "1.000000,1,1") "AdjustIfPossibleButDontSpawnIfColliding" 0 0))
  (Class|BPISpawnable|SetParent(Message) _returnvalue self)
  (return _returnvalue))