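; BP_SpawnerFloor is a child spawner that builds a looping floor from a recycled row of tiles.
; On BeginPlay it spawns tiles through the parent's SpawnActor, measures the first tile's X bounds and lines up the rest along X.
; When a tile hits the bounds, it moves behind the tracked RearTile with a fixed overlap and becomes the new rear, so tiles are reused rather than respawned.
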(event EventBeginPlay
  (|CallParentFunction)
  (for _index (range 0 (Variables|Default|GetActorsRequiredCount))
    (if (== _index 0)
      (bind _actorspawned (CallFunction|SpawnActor))
      (Variables|Default|SetRearTile _actorspawned)
      (Variables|Default|SetTileSize (* (.x (.BoxExtent (Collision|GetActorBounds _actorspawned false))) 2.0))
      (Transformation|SetActorLocation (Variables|Default|GetRearTile) (Transformation|GetActorLocation) false false)
      (else
        (bind _actorspawned_2 (CallFunction|SpawnActor))
        (Transformation|SetActorLocation _actorspawned_2 (Math|Vector|MakeVector (+ (.x (Transformation|GetActorLocation (Variables|Default|GetRearTile))) (Variables|Default|GetTileSize)) (.y (Transformation|GetActorLocation (Variables|Default|GetRearTile))) 0.0) false false)
        (Variables|Default|SetRearTile _actorspawned_2)))))

(event EventSpawnedActorHitBounds
  (params (ActorOutOfBounds :type Actor%20Object%20Reference))
  (Transformation|SetActorLocation ActorOutOfBounds (Math|Vector|MakeVector (+ (.x (Transformation|GetActorLocation (Variables|Default|GetRearTile))) (- (Variables|Default|GetTileSize) 5e+01)) (.y (Transformation|GetActorLocation (Variables|Default|GetRearTile))) (.z (Transformation|GetActorLocation (Variables|Default|GetRearTile)))) false false)
  (Variables|Default|SetRearTile ActorOutOfBounds))

(fn ConstructionScript
  (|CallParentFunction))

(fn SpawnActor
  (bind _actorspawned (|CallParentFunction))
  (return _actorspawned))