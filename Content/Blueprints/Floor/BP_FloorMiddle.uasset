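; BP_FloorMiddle is a floor piece that sizes its static mesh to fit the level's lane layout.
; On BeginPlay, after the parent logic, it checks LevelManagerRef and sets the mesh's world X and Y scale from total lane width (lane count times lane width), with a fixed Z scale.
; It also prints the computed scale as debug output; overlap, Tick and construction script add no logic.
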(event EventBeginPlay
  (bind _levelmanagerref (Variables|Default|GetLevelManagerRef))
  (bind _lanewidth (Variables|/Game/Blueprints/BP_LevelManager.BP_LevelManager_C|GetLaneWidth _levelmanagerref))
  (bind _numberoflanes (Variables|/Game/Blueprints/BP_LevelManager.BP_LevelManager_C|GetNumberOfLanes _levelmanagerref))
  (bind _returnvalue (* _numberoflanes _lanewidth))
  (bind _returnvalue_2 (/ _returnvalue 75.0))
  (|CallParentFunction)
  (Utilities|IsValid _levelmanagerref
    (:Is%20Valid
      (Transformation|SetWorldScale3D (Variables|Default|GetStaticMesh) (Math|Vector|MakeVector _returnvalue_2 _returnvalue_2 0.5))
      (Development|PrintString (Utilities|String|ToString(Float) _returnvalue_2)))))

(event Collision|EventActorBeginOverlap
  (params (OtherActor :type Actor%20Object%20Reference)))

(event EventTick
  (params (DeltaSeconds :type Float%20%28single-precision%29))
  (|CallParentFunction DeltaSeconds) ; This node is disabled and will not be called.\nDrag off pins to build functionality.
)

(fn ConstructionScript
  (|CallParentFunction))