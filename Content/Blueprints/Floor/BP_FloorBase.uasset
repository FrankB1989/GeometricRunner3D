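; BP_FloorBase is a floor piece, apparently a base Blueprint, that keeps a reference to the spawner it belongs to.
; On BeginPlay it caches the level manager if one is valid.
; RandomizeCurve sets a random Z in the mesh materials' CurveDirection vector parameter, so any curve effect comes from the material rather than the geometry.
; SetParent and ReturnParent store and expose the parent spawner.
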(event EventBeginPlay
  (bind (_levelmanager _isvalid_) (CallFunction|GetLevelManagerFunction))
  (if _isvalid_
    (Variables|Default|SetLevelManagerRef _levelmanager)))

(event EventTick
  (params (DeltaSeconds :type Float%20%28single-precision%29)))

(fn ConstructionScript)

(fn RandomizeCurve
  (Rendering|Material|SetVectorParameterValueonMaterials (Variables|Default|GetStaticMesh) "CurveDirection" (Math|Vector|MakeVector 0.0 0.0 (Math|Random|RandomFloatinRange -1.0 1.0))))

(fn ReturnParent
  (return (Variables|Default|GetParentSpawner)))

(fn SetParent
  (params (Parent :type BP%20Spawner%20Base%20Object%20Reference))
  (Variables|Default|SetParentSpawner Parent))