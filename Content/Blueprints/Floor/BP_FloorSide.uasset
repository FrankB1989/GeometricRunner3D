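; BP_FloorSide is a floor-side actor that builds a randomized cluster of static mesh instances inside a box volume.
; The construction script adds a small fixed number of instances to an InstancedStaticMesh at random points within the Box component's bounds.
; Each instance gets random X and Y scales between MinXY and MaxXY and a wider, hardcoded random Z range.
; The event graph holds only disabled default events, so nothing runs during play.
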(event EventBeginPlay
  (|CallParentFunction) ; This node is disabled and will not be called.\nDrag off pins to build functionality.
)

(event Collision|EventActorBeginOverlap
  (params (OtherActor :type Actor%20Object%20Reference)))

(event EventTick
  (params (DeltaSeconds :type Float%20%28single-precision%29))
  (|CallParentFunction DeltaSeconds) ; This node is disabled and will not be called.\nDrag off pins to build functionality.
)

(fn ConstructionScript
  (bind _box (Variables|Default|GetBox))
  (bind _maxxy (Variables|Default|GetMaxXY))
  (bind _minxy (Variables|Default|GetMinXY))
  (bind (_origin _boxextent) (Collision|GetComponentBounds _box))
  (|CallParentFunction)
  (for _index (range 0 10)
    (Components|InstancedStaticMesh|AddInstance (Variables|Default|GetInstancedStaticMesh) (Math|Transform|MakeTransform (Math|Random|RandomPointinBoundingBox _origin _boxextent) "0, 0, 0" (Math|Vector|MakeVector (Math|Random|RandomFloatinRange _minxy _maxxy) (Math|Random|RandomFloatinRange _minxy _maxxy) (Math|Random|RandomFloatinRange 2.0 2e+01))))))