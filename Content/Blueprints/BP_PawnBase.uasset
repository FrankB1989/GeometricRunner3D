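; BP_PawnBase is a pawn base Blueprint that sets up lane state for lane-based gameplay.
; On BeginPlay it looks up the Level Manager and caches the reference and lane width.
; It sets the current lane to half the manager's lane count plus one, or prints an error if no manager is found.
; It contains no movement, overlap or tick logic.
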(event EventBeginPlay
  (bind _output (Utilities|GetLevelManager)
    (:Is%20Valid
      (Variables|Default|SetLevelManagerRef _output)
      (Variables|Default|SetCurrentLane (+ (/ (Variables|/Game/Blueprints/BP_LevelManager.BP_LevelManager_C|GetNumberOfLanes (Variables|Default|GetLevelManagerRef)) 2) 1))
      (Variables|Default|SetLaneWidthRef (Variables|/Game/Blueprints/BP_LevelManager.BP_LevelManager_C|GetLaneWidth (Variables|Default|GetLevelManagerRef))))
    (:Is%20Not%20Valid
      (Development|PrintString "No Level Manager Find in Project"))))

(event Collision|EventActorBeginOverlap
  (params (OtherActor :type Actor%20Object%20Reference)))

(event EventTick
  (params (DeltaSeconds :type Float%20%28single-precision%29)))

(fn ConstructionScript)